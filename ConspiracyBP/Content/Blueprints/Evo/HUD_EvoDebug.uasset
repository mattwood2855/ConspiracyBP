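; HUD_EvoDebug is a debug HUD that draws the state of every BP_EvoPhone actor as screen text.
; Each DrawHUD call finds all phones, loops over their Apps and switches on RunningApp.
; By default it lists app names as a main menu, highlighting SelectedApp in green.
; When RunningApp is 0, it draws fixed, color-coded Easy, Normal and hard difficulty labels, with no selection highlight.
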(event `self.ReceiveBeginPlay`)

(event `self.ReceiveActorBeginOverlap`
  (params (OtherActor :type "Actor Object Reference")))

(event `self.ReceiveTick`
  (params (DeltaSeconds :type "Float (single-precision)")))

(event `self.ReceiveDrawHUD`
  (params (SizeX :type Integer) (SizeY :type Integer))
  (bind _outactors (`GameplayStatics.GetAllActorsOfClass` "/Game/Blueprints/Evo/BP_EvoPhone.BP_EvoPhone_C"))
  (for _array_element _outactors
    (for (_array_element_2 _array_index) (`/Game/Blueprints/Evo/BP_EvoPhone.Apps` _array_element)
      (switch `int` (`/Game/Blueprints/Evo/BP_EvoPhone.RunningApp` _array_element)
        (:`Default`
          ;[1 1 1] Main Menu
          (if (== _array_index (`/Game/Blueprints/Evo/BP_EvoPhone.SelectedApp` _array_element))
            (bind _name (break `/Game/Blueprints/Evo/S_EvoApp` _array_element_2))
            (bind _returnvalue (* _array_index 20.0))
            (`self.DrawText` _name (struct :`G` 0.765 :`B` 0.138819 :`A` 1.0) 0.0 _returnvalue)
            (else
              (`self.DrawText` _name (struct :`R` 0.021959 :`G` 0.025 :`B` 0.02452 :`A` 1.0) 0.0 _returnvalue))))
        (:`0`
          ;[1 1 1] Difficulty Selection
          (`self.DrawText` "Easy" (struct :`G` 0.765 :`B` 0.138819 :`A` 1.0))
          (`self.DrawText` "Normal" (struct :`R` 0.885 :`G` 0.365081 :`B` 0.075225 :`A` 1.0) 0.0 20.0)
          (`self.DrawText` "hard" (struct :`R` 0.765 :`G` 0.072201 :`B` 0.02102 :`A` 1.0) 0.0 40.0))))))

(fn `UserConstructionScript`)