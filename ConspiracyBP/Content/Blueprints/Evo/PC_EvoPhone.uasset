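; PC_EvoPhone, apparently a player controller, handles input for navigating and launching apps on BP_EvoPhone actors.
; The Down and Up actions increment and decrement SelectedApp, with no clamping or wrapping here, and Select copies SelectedApp into RunningApp.
; Each press looks up every BP_EvoPhone with GetAllActorsOfClass and writes to all of them directly, so all phones receive the same input.
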(event `self.ReceiveBeginPlay`)

(event `self.ReceiveTick`
  (params (DeltaSeconds :type "Float (single-precision)")))

(event `InputAction|Down`
  (params (Key :type "Key Structure" :default "AnyKey"))
  (:`Pressed`
    (bind _outactors (`GameplayStatics.GetAllActorsOfClass` "/Game/Blueprints/Evo/BP_EvoPhone.BP_EvoPhone_C"))
    (for _array_element _outactors
      (set `/Game/Blueprints/Evo/BP_EvoPhone.SelectedApp` (+ (`/Game/Blueprints/Evo/BP_EvoPhone.SelectedApp` _array_element) 1) _array_element))))

(event `InputAction|Up`
  (params (Key :type "Key Structure" :default "AnyKey"))
  (:`Pressed`
    (bind _outactors (`GameplayStatics.GetAllActorsOfClass` "/Game/Blueprints/Evo/BP_EvoPhone.BP_EvoPhone_C"))
    (for _array_element _outactors
      (set `/Game/Blueprints/Evo/BP_EvoPhone.SelectedApp` (+ (`/Game/Blueprints/Evo/BP_EvoPhone.SelectedApp` _array_element) -1) _array_element))))

(event `InputAction|Select`
  (params (Key :type "Key Structure" :default "AnyKey"))
  (:`Pressed`
    (bind _outactors (`GameplayStatics.GetAllActorsOfClass` "/Game/Blueprints/Evo/BP_EvoPhone.BP_EvoPhone_C"))
    (for _array_element _outactors
      (set `/Game/Blueprints/Evo/BP_EvoPhone.RunningApp` (`/Game/Blueprints/Evo/BP_EvoPhone.SelectedApp` _array_element) _array_element))))

(fn `UserConstructionScript`)